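; Enemy actor Blueprint that moves back and forth along the world Y axis.
; Each Tick offsets its location at a constant speed scaled by delta time and a DirectionY sign, without sweeping for collisions.
; DirectionY flips when the actor passes fixed world-space bounds either side of Y zero, so the path is not relative to its spawn point.
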(event EventTick
  (params (DeltaSeconds :type Float%20%28single-precision%29))
  (bind _returnvalue (Transformation|GetActorLocation))
  (bind _y (Math|Vector|BreakVector _returnvalue))
  (Transformation|SetActorLocation (+ (* (* "0,50.000000, 0" DeltaSeconds) (* "0,1.000000, 0" (Variables|Default|GetDirectionY))) (Transformation|GetActorLocation)) false false)
  (if (> _y 1e+02)
    (Variables|Default|SetDirectionY -1.0)
    (elif (< _y -1e+02)
      (Variables|Default|SetDirectionY 1.0))))

(fn ConstructionScript)