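; Player actor for a shooter that slides sideways with the mouse, fires bullets and explodes visually when hit.
; MouseX offsets its location along the Y axis without sweep, scaled by the axis value.
; Left click spawns a PlayerBulletBlueprint at the actor's location with X scaled down by multiplication, not a fixed offset.
; Any actor overlap spawns an explosion effect at its location, with no damage or destroy logic.
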(event Collision|EventActorBeginOverlap
  (params (OtherActor :type Actor%20Object%20Reference))
  ;[1 1 1] 弾が当たった時の処理
  (Game|SpawnActorfromClass "/Game/StarterContent/Blueprints/Blueprint_Effect_Explosion.Blueprint_Effect_Explosion_C" (Math|Conversions|ToTransform(Vector) (Transformation|GetActorLocation)) "Undefined" 0 0))

(event Input|MouseEvents|MouseX
  (params (AxisValue :type Float%20%28single-precision%29))
  ;[1 1 1] 移動
  (Transformation|SetActorLocation (+ (* "0,10.000000, 0" AxisValue) (Transformation|GetActorLocation)) false false))

(event Input|MouseEvents|LeftMouseButton
  (params (Key :type Key%20Structure :default "AnyKey"))
  ;[1 1 1] 弾の発射
  (:Pressed
    (Game|SpawnActorfromClass "/Game/Blueprints/PlayerBulletBlueprint.PlayerBulletBlueprint_C" (Math|Conversions|ToTransform(Vector) (* (Transformation|GetActorLocation) "0.800000,1.000000,1.000000")) "Undefined" 0 0)))

(fn ConstructionScript)